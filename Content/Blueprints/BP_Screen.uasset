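; BP_Screen is an in-world player screen that displays that player's buildings, selected-building details, economy and population, plus opponent building info.
; It polls by timer for the indexed player's BP_PlayerState, then registers itself as its Screen.
; Child meshes become indexed icon slots, with changes mirrored to the linked EnemyScreen.
; Selecting an icon maps its index to the player's Buildings and fills the text renders.
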(event Custom|GetPlayerState
  (bind _playerindex (Variables|Default|GetPlayerIndex))
  (bind _returnvalue (Game|GetPlayerState _playerindex))
  (Utilities|IsValid _returnvalue
    (:Is%20Valid
      (bind _asbp_player_state (Utilities|Casting|CastToBP_PlayerState _returnvalue))
      (bind _output_get (Variables|Default|SetPlayerState _asbp_player_state))
      (Utilities|Time|ClearandInvalidateTimerbyHandle (Variables|Default|GetTimerHandle))
      (Variables|/Game/Blueprints/Player/BP_PlayerState.BP_PlayerState_C|SetScreen _output_get self))))

(event Custom|UpdateScreenOponentBuildingIcon
  (params (Index :type Integer) (Icon :type Material%20Instance%20Object%20Reference))
  (Rendering|Material|SetMaterial (Utilities|Array|Get(acopy) (Variables|Default|GetEnemyBuildingsOnSceen) Index) 0 Icon))

(event Custom|UpdateSelectedBuildingIconText
  (if (Utilities|IsValid (stale Custom|SelectABuilding _output_get))
    (if (<= (Variables|/Game/Blueprints/Buildings/BP_Building.BP_Building_C|GetHealth (stale Custom|SelectABuilding _output_get)) 0.0)
      (Rendering|Material|SetMaterial (Variables|Default|GetIconInfo) 0 "/Game/Art/Sprites/BuildingImages/BuildingImageMaterial/M_DestroyedBuilding_Inst.M_DestroyedBuilding_Inst"))
    (if (Utilities|IsValid (stale Custom|SelectABuilding _output_get))
      (Rendering|Components|TextRender|SetText (Variables|Default|GetTextRenderBName) (Utilities|Text|ToText(String) (Utilities|String|EnumtoString (Variables|/Game/Blueprints/Buildings/BP_Building.BP_Building_C|GetBuildingType (stale Custom|SelectABuilding _output_get)))))
      (Rendering|Components|TextRender|SetText (Variables|Default|GetTextRenderBtier) (Utilities|Text|ToText(String) (Utilities|String|Append "Tier: " (Utilities|String|ToString(Integer) (Variables|/Game/Blueprints/Buildings/BP_Building.BP_Building_C|GetTier (stale Custom|SelectABuilding _output_get))))))
      (bind _newprice (Default|UpgradePriceReduction (Variables|Default|GetPlayerState) (.price (Utilities|Array|Get(acopy) (Variables|/Game/Blueprints/Buildings/BP_Building.BP_Building_C|GetTiers (stale Custom|SelectABuilding _output_get)) (Variables|/Game/Blueprints/Buildings/BP_Building.BP_Building_C|GetTier (stale Custom|SelectABuilding _output_get))))))
      (Rendering|Components|TextRender|SetText (Variables|Default|GetTextRenderUpgradeInfo) (Utilities|Text|ToText(String) (Utilities|String|Append "Price: " (Utilities|String|ToString(Integer) _newprice))))
      (Rendering|Components|TextRender|SetText (Variables|Default|GetTextRenderBHealth) (Utilities|Text|ToText(String) (Utilities|String|Append "Health: " (Utilities|String|ToString(Float) (Variables|/Game/Blueprints/Buildings/BP_Building.BP_Building_C|GetHealth (stale Custom|SelectABuilding _output_get))) " / " (Utilities|String|ToString(Float) (.maxhealth (Utilities|Array|Get(acopy) (Variables|/Game/Blueprints/Buildings/BP_Building.BP_Building_C|GetTiers (stale Custom|SelectABuilding _output_get)) (- (Variables|/Game/Blueprints/Buildings/BP_Building.BP_Building_C|GetTier (stale Custom|SelectABuilding _output_get)) 1)))))))
      (Rendering|Components|TextRender|SetText (Variables|Default|GetTextRenderBPop) (Utilities|Text|ToText(String) (Utilities|String|Append "Population: " (Utilities|String|ToString(Integer) (Variables|/Game/Blueprints/Buildings/BP_Building.BP_Building_C|GetPopulation (stale Custom|SelectABuilding _output_get))) " / " (Utilities|String|ToString(Integer) (.maxpopulation (Utilities|Array|Get(acopy) (Variables|/Game/Blueprints/Buildings/BP_Building.BP_Building_C|GetTiers (stale Custom|SelectABuilding _output_get)) (- (Variables|/Game/Blueprints/Buildings/BP_Building.BP_Building_C|GetTier (stale Custom|SelectABuilding _output_get)) 1)))))))
      (Rendering|Components|TextRender|SetText (Variables|Default|GetTextRenderBDesc) (.description (Utilities|Array|Get(acopy) (Variables|/Game/Blueprints/Buildings/BP_Building.BP_Building_C|GetTiers (stale Custom|SelectABuilding _output_get)) (- (Variables|/Game/Blueprints/Buildings/BP_Building.BP_Building_C|GetTier (stale Custom|SelectABuilding _output_get)) 1)))))))

(event Custom|SetupBuildingIcons
  (for _array_element (Components|GetChildrenComponents (Variables|Default|GetScreenBuildings) false)
    (bind _asstatic_mesh_component (Utilities|Casting|CastToStaticMeshComponent _array_element))
    (Utilities|Array|Add (Variables|Default|GetBuildingsOnScreen) _asstatic_mesh_component))
  (for _array_element_2 (Components|GetChildrenComponents (Variables|Default|GetScreenEnemyStats) false)
    (bind _asstatic_mesh_component_2 (Utilities|Casting|CastToStaticMeshComponent _array_element_2))
    (Utilities|Array|Add (Variables|Default|GetEnemyBuildingsOnSceen) _asstatic_mesh_component_2)))

(event Custom|ChangeBuildingIcon
  (params (Icon :type Material%20Instance%20Object%20Reference) (Glow :type Material%20Instance%20Object%20Reference) (Index :type Integer))
  (bind _buildingsonscreen (Variables|Default|GetBuildingsOnScreen))
  (bind _output (Utilities|Array|Get(acopy) _buildingsonscreen Index))
  (Rendering|Material|SetMaterial _output 0 Icon)
  (for _array_element (Components|GetChildrenComponents _output false)
    (bind _asstatic_mesh_component (Utilities|Casting|CastToStaticMeshComponent _array_element))
    (Rendering|Material|SetMaterial _asstatic_mesh_component 0 Glow)
    (CallFunction|UpdateScreenOponentBuildingIcon (Variables|Default|GetEnemyScreen) Index Icon)))

(event Custom|UpdateScreenNumberOponentBuildings
  (params (Amount :type Integer))
  (Rendering|Components|TextRender|SetText (Variables|Default|GetTextRendeEnemyBCurrent) (Utilities|Text|ToText(Integer) Amount)))

(event Custom|SelectABuilding
  (params (Icon :type Static%20Mesh%20Component%20Object%20Reference))
  (bind _buildingsonscreen (Variables|Default|GetBuildingsOnScreen))
  (bind _playerstate (Variables|Default|GetPlayerState))
  (bind _returnvalue (Utilities|Array|FindItem _buildingsonscreen Icon))
  (if (Utilities|Array|IsValidIndex _buildingsonscreen _returnvalue)
    (Rendering|Material|SetMaterial (Variables|Default|GetIconInfo) 0 (Rendering|Material|GetMaterial (Utilities|Array|Get(acopy) _buildingsonscreen _returnvalue) 0))
    (bind _output_get (Variables|Default|SetSelectedBuilding (Utilities|Array|Get(acopy) (Variables|/Game/Blueprints/Player/BP_PlayerState.BP_PlayerState_C|GetBuildings _playerstate) _returnvalue)))
    (if (Utilities|IsValid _output_get)
      (Rendering|Components|TextRender|SetText (Variables|Default|GetTextRenderBName) (Utilities|Text|ToText(String) (Utilities|String|EnumtoString (Variables|/Game/Blueprints/Buildings/BP_Building.BP_Building_C|GetBuildingType _output_get))))
      (Rendering|Components|TextRender|SetText (Variables|Default|GetTextRenderBtier) (Utilities|Text|ToText(String) (Utilities|String|Append "Tier: " (Utilities|String|ToString(Integer) (Variables|/Game/Blueprints/Buildings/BP_Building.BP_Building_C|GetTier _output_get)))))
      (bind _newprice (Default|UpgradePriceReduction _playerstate (.price (Utilities|Array|Get(acopy) (Variables|/Game/Blueprints/Buildings/BP_Building.BP_Building_C|GetTiers _output_get) (Variables|/Game/Blueprints/Buildings/BP_Building.BP_Building_C|GetTier _output_get)))))
      (Rendering|Components|TextRender|SetText (Variables|Default|GetTextRenderUpgradeInfo) (Utilities|Text|ToText(String) (Utilities|String|Append "Price: " (Utilities|String|ToString(Integer) _newprice))))
      (Rendering|Components|TextRender|SetText (Variables|Default|GetTextRenderBHealth) (Utilities|Text|ToText(String) (Utilities|String|Append "Health: " (Utilities|String|ToString(Float) (Variables|/Game/Blueprints/Buildings/BP_Building.BP_Building_C|GetHealth _output_get)) " / " (Utilities|String|ToString(Float) (.maxhealth (Utilities|Array|Get(acopy) (Variables|/Game/Blueprints/Buildings/BP_Building.BP_Building_C|GetTiers _output_get) (- (Variables|/Game/Blueprints/Buildings/BP_Building.BP_Building_C|GetTier _output_get) 1)))))))
      (Rendering|Components|TextRender|SetText (Variables|Default|GetTextRenderBPop) (Utilities|Text|ToText(String) (Utilities|String|Append "Population: " (Utilities|String|ToString(Integer) (Variables|/Game/Blueprints/Buildings/BP_Building.BP_Building_C|GetPopulation _output_get)) " / " (Utilities|String|ToString(Integer) (.maxpopulation (Utilities|Array|Get(acopy) (Variables|/Game/Blueprints/Buildings/BP_Building.BP_Building_C|GetTiers _output_get) (- (Variables|/Game/Blueprints/Buildings/BP_Building.BP_Building_C|GetTier _output_get) 1)))))))
      (Rendering|Components|TextRender|SetText (Variables|Default|GetTextRenderBDesc) (.description (Utilities|Array|Get(acopy) (Variables|/Game/Blueprints/Buildings/BP_Building.BP_Building_C|GetTiers _output_get) (- (Variables|/Game/Blueprints/Buildings/BP_Building.BP_Building_C|GetTier _output_get) 1)))))))

(event Custom|UpdateAllBuildingIcon
  (params (Buildings :type Array%20of%20BP%20Building%20Object%20References))
  (for (_array_element _array_index) Buildings
    (CallFunction|ChangeBuildingIcon (Variables|/Game/Blueprints/Buildings/BP_Building.BP_Building_C|GetIcon _array_element) (Variables|/Game/Blueprints/Buildings/BP_Building.BP_Building_C|GetIconGlow _array_element) _array_index)))

(event Custom|UpdateEnemyScreenNumberOfBuildings
  (params (Number :type Integer))
  (CallFunction|UpdateScreenNumberOponentBuildings (Variables|Default|GetEnemyScreen) Number))

(event Custom|UpdateCashMoneyTexts
  (params (CashMoney :type Integer64) (TaxPerPop :type Integer64) (TaxMulti :type Float%20%28double-precision%29) (IncomePerRound :type Integer64))
  (Rendering|Components|TextRender|SetText (Variables|Default|GetTextRenderTotalCashMoney) (Utilities|Text|ToText(String) (Utilities|String|Append "Cash Money: " (Utilities|String|ToString(Text) (Utilities|Text|ToText(String) CashMoney)))))
  (Rendering|Components|TextRender|SetText (Variables|Default|GetTextRenderTaxesPerPerson) (Utilities|Text|ToText(String) (Utilities|String|Append "Tax Per Population: " (Utilities|String|ToString(Text) (Utilities|Text|ToText(String) TaxPerPop)))))
  (Rendering|Components|TextRender|SetText (Variables|Default|GetTextRendermulti) (Utilities|Text|ToText(String) (Utilities|String|Append "Tax Multiplier: " (Utilities|String|ToString(Float) TaxMulti))))
  (Rendering|Components|TextRender|SetText (Variables|Default|GetTextRenderTotalIncomePerRound) (Utilities|Text|ToText(String) (Utilities|String|Append "Income Per Round: " (Utilities|String|ToString(Text) (Utilities|Text|ToText(String) IncomePerRound))))))

(event Custom|UpdatePopulationText
  (params (Population :type Integer64))
  (Rendering|Components|TextRender|SetText (Variables|Default|GetTextRenderTotalPopulation) (Utilities|Text|ToText(String) (Utilities|String|Append "Total Population: " (Utilities|String|ToString(Text) (Utilities|Text|ToText(String) Population))))))

(event EventBeginPlay
  (Actor|SetOwner (Game|GetPlayerController (Variables|Default|GetPlayerIndex)))
  (CallFunction|SetupBuildingIcons)
  (if (not (Utilities|Time|IsTimerActivebyHandle (Variables|Default|GetTimerHandle)))
    (bind _returnvalue (Utilities|Time|SetTimerbyEvent (EventDispatchers|CreateEvent :!event Custom|GetPlayerState) 0.1 true))
    (Variables|Default|SetTimerHandle _returnvalue)))

(fn ConstructionScript)