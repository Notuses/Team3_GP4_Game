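; Actor component for mouse selection, built to highlight its owner's static mesh on hover and toggle a targeted state on click.
; Hover handlers switch the mesh's custom depth, and clicks swap material slot 0 between green and red.
; BeginPlay is empty and the code that finds the mesh and binds the owner's cursor events is disconnected, so it never runs.
; A temporary InBuildingMode event destroys the component.
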(event Custom|OnMouseClicked
  (params (TouchedActor :type Actor%20Object%20Reference) (ButtonPressed :type Key%20Structure :default "None"))
  (bind _staticmeshref (Variables|Default|GetStaticMeshRef))
  (Variables|Default|SetTargeted (not (Variables|Default|GetTargeted)))
  (Utilities|IsValid (Variables|Default|GetStaticMeshRef)
    (:Is%20Valid
      (if (Variables|Default|GetTargeted)
        (Rendering|Material|SetMaterial _staticmeshref 0 "/AnimationSharing/AnimSharingGreen.AnimSharingGreen")
        (else
          (Rendering|Material|SetMaterial _staticmeshref 0 "/AnimationSharing/AnimSharingRed.AnimSharingRed"))))))

(event Custom|MouseHoverBegins
  (params (TouchedActor :type Actor%20Object%20Reference))
  (Rendering|SetRenderCustomDepth (Variables|Default|GetStaticMeshRef) true))

(event Custom|MouseHoverEnds
  (params (TouchedActor :type Actor%20Object%20Reference))
  (Rendering|SetRenderCustomDepth (Variables|Default|GetStaticMeshRef) false))

(event Custom|CustomEvent_0)

(event Custom|InBuildingMode
  ;[1 1 1] TEMP
  (Components|DestroyComponent))

(event EventBeginPlay)