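; Actor component for placeable buildings that flags whether the owner's current position is a valid placement.
; It calls UpdateState on BeginPlay and whenever the owner begins or ends an overlap, with both events sharing one handler.
; UpdateState sets ValidPlacement when no actors overlap the owner, then swaps the first two material slots on every owner static mesh to the valid or invalid material.
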(event Custom|CustomEvent_0
  (params (OverlappedActor :type Actor%20Object%20Reference) (OtherActor :type Actor%20Object%20Reference))
  (CallFunction|UpdateState))

(event EventBeginPlay
  (bind _returnvalue (Components|GetOwner))
  (Collision|BindEventtoOnActorBeginOverlap _returnvalue (delegate Custom|CustomEvent_0))
  (EventDispatchers|AssignOnActorEndOverlap _returnvalue (delegate Custom|CustomEvent_0))
  (CallFunction|UpdateState))

(fn UpdateState
  (bind _validplacementmat (Variables|Default|GetValidPlacementMat))
  (bind _invalidplacementmat (Variables|Default|GetInvalidPlacementMat))
  (Variables|Default|SetValidPlacement (== (Utilities|Array|Length (Collision|GetOverlappingActors (Components|GetOwner) "/Script/Engine.Actor" :!class /Script/Engine.Actor)) 0))
  (for _array_element (Actor|GetComponentsByClass (Components|GetOwner) "/Script/Engine.StaticMeshComponent")
    (if (Variables|Default|GetValidPlacement)
      (Rendering|Material|SetMaterial _array_element 0 _validplacementmat)
      (Rendering|Material|SetMaterial _array_element 1 _validplacementmat)
      (else
        (Rendering|Material|SetMaterial _array_element 0 _invalidplacementmat)
        (Rendering|Material|SetMaterial _array_element 1 _invalidplacementmat)))))