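; Casino is a building Blueprint that assigns itself a random tax multiplier.
; On BeginPlay, after the parent logic, it rolls a value between the minimum and maximum increase bounds, provided Health is above zero.
; The roll is rounded to two decimal places and stored as the current multiplier through a separate setter event.
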(event Custom|RandomizeCasinoTax
  (if (> (Variables|Default|GetHealth) 0.0)
    (CallFunction|SetCasinoTaxMulti (/ (Math|Conversions|ToFloat(Integer) (Math|Float|Round (* (Math|Random|RandomFloatinRange (Variables|Default|GetTaxMultiplierIncreaseMin) (Variables|Default|GetTaxMultiplierIncreaseMax)) 1e+02))) 1e+02))))

(event Custom|SetCasinoTaxMulti
  (params (TaxMulti :type Float%20%28double-precision%29))
  (Variables|Default|SetTaxMultiplierCurrent TaxMulti))

(event EventBeginPlay
  (|CallParentFunction)
  (CallFunction|RandomizeCasinoTax))

(fn ConstructionScript
  (|CallParentFunction))