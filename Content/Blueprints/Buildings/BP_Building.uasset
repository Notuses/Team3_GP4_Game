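; Tiered, destructible building actor with health and population, backed by a Chaos geometry collection.
; BeginPlay applies tier stats, binds the break event and registers an anchor field picked by comparing distances as an initialization field.
; Damage plays a sound and enables physics at zero health; breaking removes the static mesh and deregisters the building from BP_PlayerState.
; ChangeTier adjusts health and population by the difference between tiers.
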(event Custom|TakeDamage
  (params (Damage :type Float%20%28double-precision%29))
  (Audio|SpawnSoundatLocation "/Game/SFX/BuildingDestroyed.BuildingDestroyed" (Transformation|GetActorLocation self) "0, 0, 0" 1.0 1.0 0.0 0 0)
  (CallFunction|SetCurrentHealth (- (Variables|BuildingStats|GetHealth) Damage)))

(event Custom|SetCurrentPopulation
  (params (Population :type Integer64))
  (Variables|BuildingStats|SetPopulation Population))

(event Custom|EnableSimulatePhysics
  (Physics|SetSimulatePhysics (stale EventBeginPlay _output_get) true))

(event Custom|BreakEvent
  (params (BreakEvent :type Chaos%20Break%20Event%20Structure%20%28by%20ref%29))
  (EventDispatchers|UnbindEventfromOnChaosBreakEvent (stale EventBeginPlay _output_get) (delegate Custom|BreakEvent))
  (Components|DestroyComponent (Actor|GetComponentbyClass "/Script/Engine.StaticMeshComponent"))
  (Default|RemoveBuilding (.AsBP%20Player%20State (Utilities|Casting|CastToBP_PlayerState (Game|GetPlayerState (Variables|Default|GetPlayerIndex)))) self))

(event Custom|CHANGETHETIER
  (params (TIER :type Integer))
  (CallFunction|ChangeTier TIER))

(event Custom|SetCurrentHealth
  (params (Health :type Float%20%28double-precision%29))
  (bind _output_get (Variables|BuildingStats|SetHealth Health))
  (if (<= _output_get 0.0)
    (CallFunction|EnableSimulatePhysics)))

(event Custom|AddBonusHealth
  (params (BonusHp :type Float%20%28double-precision%29)))

(event EventBeginPlay
  (bind _tier (CallFunction|GetTier))
  (CallFunction|SetCurrentHealth (.maxhealth _tier))
  (Variables|BuildingStats|SetPopulation (.maxpopulation _tier))
  (bind _output_get (Variables|Default|SetGeoCollection (Actor|GetComponentbyClass "/Script/GeometryCollectionEngine.GeometryCollectionComponent")))
  (bind _anchor (CallFunction|FindAnchorField))
  (Utilities|Array|SetArrayElem (Variables|/Script/GeometryCollectionEngine.GeometryCollectionComponent|GetInitializationFields _output_get) 0 _anchor)
  (Class|GeometryCollectionComponent|SetNotifyBreaks _output_get true)
  (EventDispatchers|AssignOnChaosBreakEvent _output_get (delegate Custom|BreakEvent)))

(fn ConstructionScript)

(fn FindAnchorField
  (bind _outactors (Actor|GetAllActorsOfClass "/Engine/EditorResources/FieldNodes/FS_AnchorField_Generic.FS_AnchorField_Generic_C"))
  (for (_array_element _array_index) _outactors
    (if (== _array_index 0)
      (bind _distance (CallFunction|CheckAnchorDistance (.AsFS%20Anchor%20Field%20Generic (Utilities|Casting|CastToFS_AnchorField_Generic _array_element))))
      (Variables|Default|SetPreviousDistance _distance)
      (Variables|Default|SetAnchor (.AsFS%20Anchor%20Field%20Generic (Utilities|Casting|CastToFS_AnchorField_Generic _array_element)))
      (else
        (bind _distance_2 (CallFunction|CheckAnchorDistance (.AsFS%20Anchor%20Field%20Generic (Utilities|Casting|CastToFS_AnchorField_Generic _array_element))))
        (bind _output_get (Variables|Default|SetDistance _distance_2))
        (if (< _output_get (Variables|Default|GetPreviousDistance))
          (Variables|Default|SetAnchor (.AsFS%20Anchor%20Field%20Generic (Utilities|Casting|CastToFS_AnchorField_Generic _array_element))))
        (Variables|Default|SetPreviousDistance (Variables|Default|GetDistance)))))
  (return (Variables|Default|GetAnchor)))

(fn CheckAnchorDistance
  (params (AnchorField :type FS%20Anchor%20Field%20Generic%20Object%20Reference))
  (return (Transformation|GetDistanceTo AnchorField)))

(fn ChangeTier
  (params (Tier :type Integer))
  (bind _returnvalue (- Tier 1))
  (bind _tiers (Variables|BuildingStats|GetTiers))
  (bind _output (Utilities|Array|Get(acopy) _tiers _returnvalue))
  (bind _returnvalue_2 (- _returnvalue 1))
  (bind _output_2 (Utilities|Array|Get(acopy) _tiers _returnvalue_2))
  ;[0.3255 1 0.1567] Health
  (if (Utilities|Array|IsValidIndex _tiers _returnvalue)
    (Variables|BuildingStats|SetMaxHealth (.maxhealth _output))
    (CallFunction|SetCurrentHealth (+ (Variables|BuildingStats|GetHealth) (- (.maxhealth _output) (.maxhealth _output_2))))
    ;[0.8803 1 0.2319] Population
    (Variables|BuildingStats|SetMaxPopulation (.maxpopulation _output))
    (CallFunction|SetCurrentPopulation (+ (Variables|BuildingStats|GetPopulation) (- (.maxpopulation _output) (.maxpopulation _output_2))))
    (bind _output_get (Variables|BuildingStats|SetTier Tier))
    ;[1 0 0.1512] Debug Text
    (if (Variables|Default|GetDebugText)
      (Development|PrintString (Utilities|String|Append (Utilities|String|EnumtoString (Variables|BuildingStats|GetBuildingType)) " upgraded to Tier " (Utilities|String|ToString(Integer) _output_get)) true true "(R=0.000000,G=0.114583,B=0.458333,A=1.000000)" 1e+01))))

(fn GetTier
  (bind _tiers (Variables|BuildingStats|GetTiers))
  (bind _tier (Variables|BuildingStats|GetTier))
  (bind _returnvalue (- _tier 1))
  (if (Utilities|Array|IsValidIndex _tiers _returnvalue)
    (return (Utilities|Array|Get(acopy) _tiers _returnvalue))))