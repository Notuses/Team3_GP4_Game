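; Player controller for a multiplayer, turn-based trebuchet game with a building phase followed by a shooting phase.
; While building, a cursor trace moves a ghost preview over Buildable surfaces, and valid placements spawn on the server until the limit ends the phase.
; While shooting, camera traces send trebuchet and screen interactions to server events, with firing cycling turns through the game mode.
; It also creates the HUD widgets and switches input modes for building and pausing.
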(event Custom|UpdateBuildingType
  (params (BuildingIndex :type Integer))
  (bind _buildingref (Variables|BuildingVariables|GetBuildingRef))
  ;[1 1 1] Client Building phase stuff
  (Variables|BuildingVariables|SetCurrentBuildingIndex BuildingIndex)
  (Variables|BuildingVariables|SetShownBuildingPlacement (Utilities|Array|Get(acopy) (Variables|BuildingVariables|GetBuildingShowcase) BuildingIndex))
  ;;[1 1 1] Sets selected building from widget input.
  (Utilities|IsValid _buildingref
    (:Is%20Valid
      (Actor|DestroyActor _buildingref))
    (:Is%20Not%20Valid
      _))
  (CallFunction|RefreshPlaceableBuilding))

(event Custom|Client_StartTurn
  ;[1 1 1] Client Events
  (CallFunction|SetMyTurn true)
  ;;[1 1 1] temp
  (Utilities|ToggleBuildUI))

(event Custom|Client_BuildPhaseBegin
  ;[1 1 1] Client Events
  (Default|SetGameState (Variables|GameState|GetGameStateRef) "NewEnumerator2")
  (CallFunction|SetBuildingMode true)
  (Utilities|ToggleBuildUI))

(event Custom|Server_EndGame
  ;[1 1 1] temp
  (bind _asbp_game_mode (Utilities|Casting|CastToBP_GameMode (Game|GetGameMode)))
  (Default|EndGame _asbp_game_mode))

(event Custom|ENDGAMETEMP
  ;[1 1 1] temp
  (CallFunction|ServerEndGame))

(event Custom|ServerSelectOnScreen
  (params (hit :type Primitive%20Component%20Object%20Reference))
  (bind _parents (Class|SceneComponent|GetParentComponents hit))
  (bind _playerindex (Variables|Default|GetPlayerIndex))
  (bind _returnvalue (Game|GetPlayerState _playerindex))
  (bind _output (Utilities|Array|Get(acopy) _parents))
  (bind _asbp_player_state (Utilities|Casting|CastToBP_PlayerState _returnvalue))
  ;[1 1 1] Server events
  (bind _asstatic_mesh_component (Utilities|Casting|CastToStaticMeshComponent _output)
    (:then
      (Default|SelectBuildingIcon _asbp_player_state _asstatic_mesh_component))
    (:CastFailed
      (Utilities|Casting|CastToTextRenderComponent _output)
      (Default|UpgradeABuilding _asbp_player_state))))

(event Custom|Server_Interact
  (params (Trebuchet :type BP%20Trebuchet%20Current%20Object%20Reference) (InteractiveComp :type Actor%20Component%20Object%20Reference))
  (if (== (Variables|/Game/Blueprints/BP_TrebuchetCurrent.BP_TrebuchetCurrent_C|GetSM_WeightControll_IncreaseButton Trebuchet) InteractiveComp)
    (Default|IncreaseWeight Trebuchet)
    (elif (== (Variables|/Game/Blueprints/BP_TrebuchetCurrent.BP_TrebuchetCurrent_C|GetSM_WeightControll_DecreaseButton Trebuchet) InteractiveComp)
      (Default|DecreaseWeight Trebuchet)
      (else
        (if (and (Variables|/Game/Blueprints/BP_TrebuchetCurrent.BP_TrebuchetCurrent_C|GetbIsLoaded Trebuchet) (== (Variables|/Game/Blueprints/BP_TrebuchetCurrent.BP_TrebuchetCurrent_C|GetFireHandle Trebuchet) InteractiveComp))
          (bind _asbp_game_mode (Utilities|Casting|CastToBP_GameMode (Game|GetGameMode)))
          (Default|CycleTurns _asbp_game_mode))
        (Default|ServerTrebuchetInteract Trebuchet InteractiveComp)))))

(event Custom|Client_EndTurn
  ;[1 1 1] Client Events
  (CallFunction|SetMyTurn false))

(event Custom|Client_EndBuildPhase
  ;[1 1 1] Client Events
  (Default|SetGameState (Variables|GameState|GetGameStateRef) "NewEnumerator3")
  (CallFunction|SetBuildingMode false)
  (Utilities|FlowControl|DelayUntilNextTick)
  (Utilities|ToggleBuildUI)
  (CallFunction|ServerBuildPhaseEnd))

(event Custom|ToggleBuild
  (bind _gamestateref (Variables|GameState|GetGameStateRef))
  ;[1 1 1] Client Building phase stuff
  ;;[1 1 1] Toggle Building HUD and Input
  (Utilities|FlowControl|FlipFlop
    (:A
      (Default|SetGameState _gamestateref "NewEnumerator2")
      (CallFunction|SetBuildingMode true))
    (:B
      (Default|SetGameState _gamestateref "NewEnumerator3")
      (CallFunction|SetBuildingMode false)))
  (Utilities|ToggleBuildUI))

(event Custom|SpawnOnServer
  (params (BuildingSelection :type Actor%20Class%20Reference) (NewParam :type Transform))
  ;[1 1 1] Server events
  (bind _returnvalue (Game|SpawnActorfromClass BuildingSelection (Math|Transform|MakeTransform (.location NewParam) (.rotation NewParam) "1.000000,1.000000,1.000000") "AlwaysSpawn" 0 0))
  (CallFunction|AddBuilding _returnvalue))

(event Custom|AddBuilding
  (params (Building :type Actor%20Object%20Reference))
  ;[1 1 1] Server events
  ;;[1 1 1] PlayerStats
  (bind _asbp_building (Utilities|Casting|CastToBP_Building Building))
  (Variables|/Game/Blueprints/Buildings/BP_Building.BP_Building_C|SetPlayerIndex _asbp_building (Variables|Default|GetPlayerIndex))
  (Default|AddBuilding (.AsBP%20Player%20State (Utilities|Casting|CastToBP_PlayerState (Game|GetPlayerState (Variables|Default|GetPlayerIndex)))) _asbp_building))

(event Custom|SetPlayerIndex
  (params (PlayerIndex :type Integer))
  (Variables|Default|SetPlayerIndex PlayerIndex))

(event Custom|Server_BuildPhaseEnd
  ;[1 1 1] Server events
  (bind _asbp_game_mode (Utilities|Casting|CastToBP_GameMode (Game|GetGameMode)))
  (Default|BuildPhaseEnd _asbp_game_mode))

(event EventTick
  (params (DeltaSeconds :type Float%20%28single-precision%29))
  (bind _gamestateref (Variables|GameState|GetGameStateRef))
  (if (Pawn|IsLocalController)
    (Utilities|IsValid _gamestateref
      (:Is%20Valid
        (switch Utilities|FlowControl|Switch|SwitchonE_CurrentGameState (Variables|/Game/Blueprints/BP_GameState.BP_GameState_C|GetCurrentState _gamestateref)
          (:NewEnumerator2
            (CallFunction|UpdatePlacement)))))))

(event EventBeginPlay
  (if (Pawn|IsLocalController)
    (Utilities|CreatePlayerWidgets)
    (bind _asbp_game_state (Utilities|Casting|CastToBP_GameState (Game|GetGameState)))
    (Variables|GameState|SetGameStateRef _asbp_game_state)))

(event Input|ActionEvents|InputActionInteract
  (params (Key :type Key%20Structure :default "None"))
  (bind _gamestateref (Variables|GameState|GetGameStateRef))
  (:Pressed
    (Utilities|IsValid _gamestateref
      (:Is%20Valid
        (switch Utilities|FlowControl|Switch|SwitchonE_CurrentGameState (Variables|/Game/Blueprints/BP_GameState.BP_GameState_C|GetCurrentState _gamestateref)
          (:NewEnumerator2
            (if (Variables|BuildingVariables|GetBuildModeActive)
              (CallFunction|SpawnSelectedBuilding)))
          (:NewEnumerator3
            (if (Variables|Default|GetMyTurn)
              (CallFunction|Interact))))))))

(event Input|ActionEvents|InputActionMenu/Deselect
  (params (Key :type Key%20Structure :default "None"))
  (bind _self self)
  (bind _player_widget_switcher (Variables|Default|GetPlayer%20Widget%20Switcher))
  (:Pressed
    (switch Utilities|FlowControl|Switch|SwitchonE_CurrentGameState (Variables|/Game/Blueprints/BP_GameState.BP_GameState_C|GetCurrentState (Variables|GameState|GetGameStateRef))
      (:NewEnumerator0
        (Game|SetGamePaused false)
        (Default|SetGameState (Variables|GameState|GetGameStateRef) "NewEnumerator3")
        (Variables|Default|SetbShowMouseCursor false)
        (Class|WidgetSwitcher|SetActiveWidgetIndex _player_widget_switcher)
        (Input|SetInputModeGameOnly _self))
      (:NewEnumerator3
        (Game|SetGamePaused true)
        (Default|SetGameState (Variables|GameState|GetGameStateRef) "NewEnumerator0")
        (Variables|Default|SetbShowMouseCursor true)
        (Class|WidgetSwitcher|SetActiveWidgetIndex _player_widget_switcher 1)
        (Input|SetInputModeUIOnly _self (Variables|UI|GetPauseMenuRef) "DoNotLock")))))

(event Input|AxisEvents|InputAxisRotateBuilding
  (params (AxisValue :type Float%20%28single-precision%29))
  (bind _buildingref (Variables|BuildingVariables|GetBuildingRef))
  (bind _returnvalue (Transformation|GetActorRotation _buildingref))
  ;[1 1 1] Rotate selected building
  (Utilities|IsValid _buildingref
    (:Is%20Valid
      (Transformation|SetActorRotation _buildingref (Math|Rotator|MakeRotator (.roll _returnvalue) (.pitch _returnvalue) (+ (.yaw _returnvalue) (* AxisValue (Variables|BuildingVariables|GetBuildingRotationSpeed))))))))

(event Input|KeyboardEvents|1
  (params (Key :type Key%20Structure :default "None"))
  ;[1 1 1] temp
  (:Pressed
    (CallFunction|ToggleBuild)))

(event Input|KeyboardEvents|2
  (params (Key :type Key%20Structure :default "None"))
  ;[1 1 1] temp
  (:Pressed
    (CallFunction|ToggleBuild)
    (CallFunction|ServerBuildPhaseEnd)))

(fn ConstructionScript)

(fn SetBuildingMode
  (params (CanBuild :type Boolean))
  (bind _buildingref (Variables|BuildingVariables|GetBuildingRef))
  (if (== CanBuild (Variables|BuildingVariables|GetBuildModeActive))
    (return)
    (else
      (bind _output_get (Variables|BuildingVariables|SetBuildModeActive CanBuild))
      (if _output_get
        (CallFunction|RefreshPlaceableBuilding)
        (else
          (Variables|BuildingVariables|SetShownBuildingPlacement 0)
          (Utilities|IsValid _buildingref
            (:Is%20Valid
              (Actor|DestroyActor _buildingref))))))))

(fn UpdatePlacement
  (bind _self self)
  (bind _buildingref (Variables|BuildingVariables|GetBuildingRef))
  (bind (_worldlocation _worlddirection) (Game|Player|ConvertMouseLocationToWorldSpace _self))
  (bind _returnvalue (Utilities|IsValid _buildingref))
  (if (Variables|BuildingVariables|GetBuildModeActive)
    (bind _outhit (Collision|LineTraceByChannel _worldlocation (+ _worldlocation (* _worlddirection 1.5e+04)) "TraceTypeQuery3" false 0 "None"))
    (Utilities|IsValid (.HitActor (Collision|BreakHitResult _outhit))
      (:Is%20Valid
        (if (Actor|ActorHasTag (.HitActor (Collision|BreakHitResult _outhit)) "Buildable")
          (if _returnvalue
            (Rendering|SetActorHiddenInGame _buildingref false)
            (Transformation|SetActorLocation _buildingref (.Location (Collision|BreakHitResult _outhit)) false false))
          (else
            (if _returnvalue :!label _label
              (Rendering|SetActorHiddenInGame _buildingref true)))))
      (:Is%20Not%20Valid
        (goto _label)))
    (else
      (return))))

(fn SpawnSelectedBuilding
  (bind _buildingref (Variables|BuildingVariables|GetBuildingRef))
  (bind _maxbuildings (Variables|BuildingVariables|GetMaxBuildings))
  (bind _returnvalue (Actor|GetComponentbyClass _buildingref "/Game/Blueprints/Components/BP_PlaceableBuildingComponent.BP_PlaceableBuildingComponent_C"))
  (if (Variables|BuildingVariables|GetBuildModeActive)
    (Utilities|IsValid _buildingref
      (:Is%20Valid
        (Utilities|IsValid _returnvalue
          (:Is%20Valid
            (if (Variables|/Game/Blueprints/Components/BP_PlaceableBuildingComponent.BP_PlaceableBuildingComponent_C|GetValidPlacement _returnvalue)
              (if (< (Variables|BuildingVariables|GetCurrentBuildings) (Variables|BuildingVariables|GetMaxBuildings))
                (bind _output_get (Variables|BuildingVariables|SetSpawnBuilding (Utilities|Array|Get(acopy) (Variables|BuildingVariables|GetBuildingToSpawn) (Utilities|Array|FindItem (Variables|BuildingVariables|GetBuildingShowcase) (Variables|BuildingVariables|GetShownBuildingPlacement)))))
                (CallFunction|SpawnonServer _output_get (Transformation|GetActorTransform (Variables|BuildingVariables|GetBuildingRef)))
                (CallFunction|UpdateBuildWidget)
                (bind _output_get_2 (Variables|BuildingVariables|SetCurrentBuildings (+ (Variables|BuildingVariables|GetCurrentBuildings) 1)))
                (Rendering|Components|TextRender|SetText (Variables|/Game/UI/WBP_BuildingHeader.WBP_BuildingHeader_C|GetText_BuildingsLeft (Variables|UI|GetBuildingHeaderRef)) (Utilities|Text|ToText(String) (Utilities|String|Append "Buildings to place: " (Utilities|String|ToString(Integer) (- _maxbuildings (Variables|BuildingVariables|GetCurrentBuildings))))))
                (if (== _output_get_2 _maxbuildings)
                  (CallFunction|ClientEndBuildPhase))))))))
    (else
      (return))))

(fn RefreshPlaceableBuilding
  (bind _shownbuildingplacement (Variables|BuildingVariables|GetShownBuildingPlacement))
  (if (!= _shownbuildingplacement 0)
    (bind _returnvalue (Game|SpawnActorfromClass _shownbuildingplacement (Math|Transform|MakeTransform "0, 0,-10000.000000" "0, 0, 0" "1.010000,1.010000,1.010000") "AlwaysSpawn" 0 0))
    (bind _output_get (Variables|BuildingVariables|SetBuildingRef _returnvalue))
    (Utilities|IsValid (Actor|GetComponentbyClass _output_get "/Game/Blueprints/Components/BP_SelectionComponent.BP_SelectionComponent_C")
      (:Is%20Valid
        (Default|InBuildingMode (Actor|GetComponentbyClass _output_get "/Game/Blueprints/Components/BP_SelectionComponent.BP_SelectionComponent_C")))
      (:Is%20Not%20Valid
        _))
    (AddComponent|AddBPPlaceableBuildingComponent (Variables|BuildingVariables|GetBuildingRef))))

(fn Interact
  (bind _asbp_player (Utilities|Casting|CastToBP_Player (Pawn|GetControlledPawn)))
  (bind _outhit (Collision|LineTraceByChannel (Transformation|GetWorldLocation (Variables|/Game/Blueprints/Player/BP_Player.BP_Player_C|GetPlayerCamera _asbp_player)) (+ (Transformation|GetWorldLocation (Variables|/Game/Blueprints/Player/BP_Player.BP_Player_C|GetPlayerCamera _asbp_player)) (* (Math|Vector|GetForwardVector (Transformation|GetWorldRotation (Variables|/Game/Blueprints/Player/BP_Player.BP_Player_C|GetPlayerCamera _asbp_player))) (LocalVariables|GetInteractReach))) "TraceTypeQuery1" false 0 "None"))
  (bind _asbp_trebuchet_current (Utilities|Casting|CastToBP_TrebuchetCurrent (.HitActor (Collision|BreakHitResult _outhit)))
    (:then
      (CallFunction|ServerInteract _asbp_trebuchet_current (.HitComponent (Collision|BreakHitResult _outhit))))
    (:CastFailed
      ;[1 1 1] SCREEN SELECT BUILDING
      (if (.bBlockingHit (Collision|BreakHitResult _outhit))
        (CallFunction|ServerSelectonScreen (.HitComponent (Collision|BreakHitResult _outhit)))))))

(fn SetMyTurn
  (params (MyTurn :type Boolean))
  (bind _output_get (Variables|Default|SetMyTurn MyTurn))
  (Default|CallOnMyTurnChanged _output_get))

(fn GetPlayerIndex
  (return (Variables|Default|GetPlayerIndex)))

(fn OnRepSpawnBuilding)

(fn UpdateBuildWidget
  (Default|BuildingAdded (Variables|UI|GetBuildingWidgetRef) (Variables|BuildingVariables|GetCurrentBuildingIndex)))