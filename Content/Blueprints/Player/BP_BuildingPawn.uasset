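; BP_BuildingPawn is a player pawn that acts as a free-flying camera, presumably for a building mode.
; Move, Strafe and Up/Down axes feed movement input along the actor's forward and right vectors and world up, scaled by CameraSpeed.
; Holding right mouse enables look and turn, hides the cursor and pins it to viewport center each Tick.
; Release restores the saved cursor position, then shows the cursor after a zero-length Delay.
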(event EventBeginPlay
  (bind _asbp_player_controller (Utilities|Casting|CastToBP_PlayerController (Pawn|GetController)))
  (Variables|Default|SetPlayerController _asbp_player_controller))

(event Collision|EventActorBeginOverlap
  (params (OtherActor :type Actor%20Object%20Reference)))

(event EventTick
  (params (DeltaSeconds :type Float%20%28single-precision%29))
  (bind _returnvalue (Viewport|GetViewportSize))
  (if (Variables|Default|GetRightMouseButtonDown)
    (Class|PlayerController|SetMouseLocation (Variables|Default|GetPlayerController) (Math|Float|Truncate (/ (.x _returnvalue) 2.0)) (Math|Float|Truncate (/ (.y _returnvalue) 2.0)))))

(event Input|ActionEvents|InputActionRightMouse
  (params (Key :type Key%20Structure :default "None"))
  (bind _playercontroller (Variables|Default|GetPlayerController))
  (bind (_locationx _locationy) (Game|Player|GetMousePosition _playercontroller))
  (:Pressed
    (Variables|/Script/Engine.PlayerController|SetbShowMouseCursor (Variables|Default|GetPlayerController) false)
    (Utilities|FlowControl|Delay 0.0)
    (Variables|Default|SetRightMouseButtonDown true)
    (Variables|Default|SetMouseSavedPosition (Utilities|Struct|MakeIntPoint (Math|Float|Truncate _locationx) (Math|Float|Truncate _locationy))))
  (:Released
    (Variables|Default|SetRightMouseButtonDown false)
    (Class|PlayerController|SetMouseLocation (Variables|Default|GetPlayerController) (.x (Variables|Default|GetMouseSavedPosition)) (.y (Variables|Default|GetMouseSavedPosition)))
    (Utilities|FlowControl|Delay 0.0)
    (Variables|/Script/Engine.PlayerController|SetbShowMouseCursor (Variables|Default|GetPlayerController) true)))

(event Input|AxisEvents|InputAxisStrafe
  (params (AxisValue :type Float%20%28single-precision%29))
  (Pawn|Input|AddMovementInput (Transformation|GetActorRightVector) (* AxisValue (Variables|Default|GetCameraSpeed)) false))

(event Input|AxisEvents|InputAxisMove
  (params (AxisValue :type Float%20%28single-precision%29))
  (Pawn|Input|AddMovementInput (Transformation|GetActorForwardVector) (* AxisValue (Variables|Default|GetCameraSpeed)) false))

(event Input|AxisEvents|InputAxisUp/Down
  (params (AxisValue :type Float%20%28single-precision%29))
  (Pawn|Input|AddMovementInput (Math|Vector|VectorUp) (* AxisValue (Variables|Default|GetCameraSpeed)) false))

(event Input|AxisEvents|InputAxisLook
  (params (AxisValue :type Float%20%28single-precision%29))
  (if (Variables|Default|GetRightMouseButtonDown)
    (Pawn|Input|AddControllerPitchInput AxisValue)))

(event Input|AxisEvents|InputAxisTurn
  (params (AxisValue :type Float%20%28single-precision%29))
  (if (Variables|Default|GetRightMouseButtonDown)
    (Pawn|Input|AddControllerYawInput AxisValue)))

(fn ConstructionScript)