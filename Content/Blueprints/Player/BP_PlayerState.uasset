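; Player state for a city-building versus game, tracking one player's buildings, population, cash and loss condition.
; Adding, upgrading or destroying buildings recalculates population and refreshes the Screen; taxes scale population by summed building multipliers, with casino bonuses re-randomized after collection.
; Shops discount upgrades, and the first hospital found absorbs part of a destroyed building's population.
; Destroyed buildings stay in the array with zeroed stats; zero population triggers the GameMode's EndGame.
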(event Custom|SelectBuildingIcon
  (params (Icon :type Static%20Mesh%20Component%20Object%20Reference))
  (Default|SelectABuilding (Variables|Default|GetScreen) Icon))

(event Custom|UpgradeABuilding
  (CallFunction|UpgradeBuilding (Variables|/Game/Blueprints/BP_Screen.BP_Screen_C|GetSelectedBuilding (Variables|Default|GetScreen))))

(event Custom|SetTaxMultiplier
  (bind _taxmultiplier (CallFunction|GetTaxMultiplier))
  (bind _output_get (Variables|Economy|SetTaxMultiplier _taxmultiplier))
  (Development|PrintString (Utilities|String|ToString(Float) _output_get)))

(event Custom|CollectTaxes
  (CallFunction|TaxCollection))

(event Custom|WIN
  (bind _asbp_game_mode (Utilities|Casting|CastToBP_GameMode (Game|GetGameMode)))
  (Default|EndGame _asbp_game_mode))

(event Custom|LOOSE
  (bind _asbp_game_mode (Utilities|Casting|CastToBP_GameMode (Game|GetGameMode)))
  (Default|EndGame _asbp_game_mode))

(event Custom|WinOrLoose
  (if (Variables|Default|GetIlost)
    (CallFunction|LOOSE)
    (else
      (CallFunction|WIN))))

(event EventTick
  (params (DeltaSeconds :type Float%20%28single-precision%29))
  (bind _buildingsowned (Variables|Default|GetBuildingsOwned))
  (if (Variables|Default|GetDebugText)
    (if (Networking|IsServer)
      (Development|PrintString (Utilities|String|Append "Current Population: " (Utilities|String|ToString(Integer) (Variables|Default|GetPopulation))) true false "(R=0.056136,G=0.069068,B=0.526042,A=1.000000)" 0.0)
      (Development|PrintString (Utilities|GetDisplayName self) true false "(R=0.056136,G=0.069068,B=0.526042,A=1.000000)" 0.0)
      (for _array_element (Variables|Default|GetBuildings)
        (Development|PrintString (Utilities|GetDisplayName _array_element) true false "(R=0.776042,G=0.600524,B=0.095803,A=1.000000)" 0.0))
      (Development|PrintString "Buildings Owned:" true false "(R=0.906250,G=0.164545,B=0.028320,A=1.000000)" 0.0)
      (bind _keys (Utilities|Map|Keys _buildingsowned))
      (for _array_element_2 _keys
        (Development|PrintString (Utilities|String|Append (Utilities|String|EnumtoString _array_element_2) ": " (Utilities|String|ToString(Integer) (.Value (Utilities|Map|Find _buildingsowned _array_element_2)))) true true "(R=0.000000,G=0.660000,B=1.000000,A=1.000000)" 0.0))
      (Development|PrintString (Utilities|String|Append "CASH MONEYS: " (Utilities|String|ToString(Integer) (Variables|Economy|GetCashMoney))) true true "(R=0.958333,G=0.662132,B=0.000000,A=1.000000)" 0.0))))

(fn ConstructionScript)

(fn RemoveBuilding
  (params (Building :type BP%20Building%20Object%20Reference))
  (bind _buildings (Variables|Default|GetBuildings))
  (bind _screen (Variables|Default|GetScreen))
  (bind _buildingtype (Variables|/Game/Blueprints/Buildings/BP_Building.BP_Building_C|GetBuildingType Building))
  (bind _buildingsowned (Variables|Default|GetBuildingsOwned))
  (bind _returnvalue (Utilities|Array|FindItem _buildings Building))
  (bind (_value _returnvalue_2) (Utilities|Map|Find _buildingsowned _buildingtype))
  (if (Utilities|Array|IsValidIndex _buildings _returnvalue)
    (bind _output_get (LocalVariables|SetIndexOfDestroyedBuilding _returnvalue))
    (bind _ascasino (Utilities|Casting|CastToCasino Building)
      (:then
        (Default|SetCasinoTaxMulti _ascasino 0.0))
      (:CastFailed
        _))
    (bind _array_element (Utilities|Array|ForEachLoopwithBreak _buildings :!label _label)
      (:LoopBody
        (bind _ashospital (Utilities|Casting|CastToHospital _array_element))
        (bind _output_get_2 (LocalVariables|SetHospitalFound _ashospital))
        (Default|SetCurrentPopulation _output_get_2 (+ (Variables|/Game/Blueprints/Buildings/BP_Building.BP_Building_C|GetPopulation _output_get_2) (Class|KismetMathLibrary|ToInt64(Integer) (Math|Float|Truncate (* (Math|Conversions|ToFloat(Integer) (Variables|/Game/Blueprints/Buildings/BP_Building.BP_Building_C|GetPopulation Building)) (Utilities|Array|Get(acopy) (Variables|/Game/Blueprints/Buildings/Hospital.Hospital_C|GetBuffTiersSavePop _output_get_2) (- (Variables|/Game/Blueprints/Buildings/BP_Building.BP_Building_C|GetTier _output_get_2) 1)))))))
        (goto _label Break))
      (:Completed
        (Default|SetCurrentPopulation Building)
        (Default|SetCurrentHealth Building 0.0)
        (Variables|/Game/Blueprints/Buildings/BP_Building.BP_Building_C|SetUseTaxMultiplier Building false)
        (CallFunction|UpdatePopulation)
        (Default|ChangeBuildingIcon _screen "/Game/Art/Sprites/BuildingImages/BuildingImageMaterial/M_DestroyedBuilding_Inst.M_DestroyedBuilding_Inst" "/Game/Art/Sprites/BuildingImages/BuildingImageMaterial/M_EmptyGlow_Inst.M_EmptyGlow_Inst" _output_get)
        (Default|UpdateEnemyScreenNumberOfBuildings _screen (Utilities|Array|Length (Variables|Default|GetBuildings)))
        (CallFunction|ScreenUpdateCashMoneys)
        (if _returnvalue_2
          (if (> _value 1)
            (Utilities|Map|Add _buildingsowned _buildingtype (- _value 1))
            (else
              (Utilities|Map|Remove _buildingsowned _buildingtype)))
          (bind _lost (CallFunction|CheckifLost (Variables|/Game/Blueprints/Buildings/BP_Building.BP_Building_C|GetPlayerIndex Building)))
          (bind _output_get_3 (Variables|Default|SetIlost _lost))
          (if _output_get_3
            (CallFunction|WinorLoose))
          (if (Variables|Default|GetDebugText)
            (bind _values (Utilities|Map|Values _buildingsowned))
            (for _array_element_2 _values
              (Development|PrintString (Utilities|String|ToString(Integer) _array_element_2)))))))))

(fn AddBuilding
  (params (Building :type BP%20Building%20Object%20Reference))
  (bind _buildings (Variables|Default|GetBuildings))
  (bind _screen (Variables|Default|GetScreen))
  (bind _buildingtype (Variables|/Game/Blueprints/Buildings/BP_Building.BP_Building_C|GetBuildingType Building))
  (bind _buildingsowned (Variables|Default|GetBuildingsOwned))
  (Utilities|Array|Add _buildings Building)
  (CallFunction|UpdatePopulation)
  (Utilities|Map|Add _buildingsowned _buildingtype (+ (.Value (Utilities|Map|Find _buildingsowned _buildingtype)) 1))
  (Default|UpdateAllBuildingIcon _screen (Variables|Default|GetBuildings))
  (Default|UpdateEnemyScreenNumberOfBuildings _screen (Utilities|Array|Length _buildings))
  (CallFunction|ScreenUpdateCashMoneys)
  (if (Variables|Default|GetDebugText)
    (bind _values (Utilities|Map|Values _buildingsowned))
    (for _array_element _values
      (Development|PrintString (Utilities|String|ToString(Integer) _array_element)))))

(fn TaxCollection
  (bind _taxmultiplier (CallFunction|GetTaxMultiplier))
  (Variables|Economy|SetCashMoney (+ (Variables|Economy|GetCashMoney) (Class|KismetMathLibrary|ToInt64(Float) (* (Math|Conversions|ToFloat(Integer) (Math|Conversions|ToInteger(Byte) (* (Variables|Default|GetPopulation) (Variables|Economy|GetTaxIncomePerPop)))) _taxmultiplier))))
  (for _array_element (Variables|Default|GetBuildings)
    (bind _ascasino (Utilities|Casting|CastToCasino _array_element))
    (Default|RandomizeCasinoTax _ascasino))
  (CallFunction|ScreenUpdateCashMoneys)
  (if (Variables|Default|GetDebugText)
    (Development|PrintString (Utilities|String|Append "You collected: " (Utilities|String|ToString(Integer) (Class|KismetMathLibrary|ToInt64(Float) (* (Math|Conversions|ToFloat(Integer) (Math|Conversions|ToInteger(Byte) (* (Variables|Default|GetPopulation) (Variables|Economy|GetTaxIncomePerPop)))) _taxmultiplier))) " Cash Money from taxes!") true true "(R=0.000000,G=0.660000,B=1.000000,A=1.000000)" 1e+01)))

(fn CheckifLost
  (params (PlayerIndex :type Integer))
  (bind _population (Variables|Default|GetPopulation))
  (bind _returnvalue (<= _population 0))
  (if _returnvalue
    (return _returnvalue)))

(fn UpgradeBuilding
  (params (Building :type BP%20Building%20Object%20Reference))
  (bind _tiers (Variables|/Game/Blueprints/Buildings/BP_Building.BP_Building_C|GetTiers Building))
  (bind _tier (Variables|/Game/Blueprints/Buildings/BP_Building.BP_Building_C|GetTier Building))
  (if (Utilities|IsValid Building)
    (if (> (Variables|/Game/Blueprints/Buildings/BP_Building.BP_Building_C|GetHealth Building) 0.0)
      (if (Utilities|Array|IsValidIndex _tiers _tier)
        (bind _newprice (CallFunction|UpgradePriceReduction (.price (Utilities|Array|Get(acopy) _tiers _tier))))
        (if (>= (Variables|Economy|GetCashMoney) _newprice)
          (bind _output_get (Variables|Economy|SetCashMoney (- (stale _output_get) _newprice)))
          (Default|CHANGETHETIER Building (+ _tier 1))
          (CallFunction|UpdatePopulation)
          (CallFunction|ScreenUpdateCashMoneys)
          (Default|UpdateSelectedBuildingIconText (Variables|Default|GetScreen)))))))

(fn UpdatePopulation
  (Variables|Default|SetPopulation 0)
  (for _array_element (Variables|Default|GetBuildings)
    (bind _output_get (Variables|Default|SetPopulation (+ (stale _output_get) (Variables|/Game/Blueprints/Buildings/BP_Building.BP_Building_C|GetPopulation _array_element)))))
  (Default|UpdatePopulationText (Variables|Default|GetScreen) (Variables|Default|GetPopulation)))

(fn ScreenUpdateCashMoneys
  (bind _taxincomeperpop (Variables|Economy|GetTaxIncomePerPop))
  (bind _taxmultiplier (CallFunction|GetTaxMultiplier))
  (Default|UpdateCashMoneyTexts (Variables|Default|GetScreen) (Variables|Economy|GetCashMoney) _taxincomeperpop _taxmultiplier (Class|KismetMathLibrary|ToInt64(Float) (* (Math|Conversions|ToFloat(Integer) (* (Variables|Default|GetPopulation) _taxincomeperpop)) _taxmultiplier))))

(fn UpgradePriceReduction
  (params (Price :type Integer64))
  (for _array_element (Variables|Default|GetBuildings)
    (bind _asshop (Utilities|Casting|CastToShop _array_element))
    (bind _output_get (LocalVariables|SetPriceReductionTotal (+ (stale _output_get) (Utilities|Array|Get(acopy) (Variables|/Game/Blueprints/Buildings/Shop.Shop_C|GetBuffTierCheaperUpgrades _asshop) (- (Variables|/Game/Blueprints/Buildings/BP_Building.BP_Building_C|GetTier _asshop) 1))))))
  (return (Class|KismetMathLibrary|ToInt64(Float) (* (Math|Conversions|ToFloat(Integer) Price) (- 1.0 (LocalVariables|GetPriceReductionTotal))))))

(fn GetTaxMultiplier
  (for _array_element (Variables|Default|GetBuildings)
    (bind _ascasino (Utilities|Casting|CastToCasino _array_element)
      (:then
        (bind _output_get (LocalVariables|SetCasinoTaxBonus (+ (stale _output_get) (Variables|/Game/Blueprints/Buildings/Casino.Casino_C|GetTaxMultiplierCurrent _ascasino)))))
      (:CastFailed
        _))
    (if (Variables|/Game/Blueprints/Buildings/BP_Building.BP_Building_C|GetUseTaxMultiplier _array_element)
      (bind _output_get_2 (LocalVariables|SetTaxMultiplierTotal (+ (stale _output_get_2) (Utilities|Array|Get(acopy) (Variables|/Game/Blueprints/Buildings/BP_Building.BP_Building_C|GetTaxMultiplier _array_element) (- (Variables|/Game/Blueprints/Buildings/BP_Building.BP_Building_C|GetTier _array_element) 1)))))))
  (return (+ (LocalVariables|GetTaxMultiplierTotal) (LocalVariables|GetCasinoTaxBonus))))