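; Game mode for a two-player turn-based match with a build phase, a shoot phase and shifting wind.
; The second login starts building and randomizes wind; once both players finish, it respawns them as BP_Player at index-matched starts.
; CycleTurns swaps the active controller via client events, collects that player's taxes and nudges wind through timelines.
; Getters expose wind strength, direction and force; EndGame returns to the main menu after a delay.
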(event Custom|StartGame
  ;[1 1 1] Shoot phase
  (Default|ClientStartTurn (Utilities|PlayerinTurn)))

(event Custom|CycleTurns
  (bind _playercontroller (Utilities|PlayerinTurn))
  ;[1 1 1] Shoot phase
  (CallFunction|UpdateWindDirection)
  (CallFunction|UpdateWindStrength)
  (Default|ClientEndTurn (Utilities|PlayerinTurn))
  (Variables|Default|SetCurrentPlayersTurn (select (== (Variables|Default|GetCurrentPlayersTurn) 0) 1 0))
  (bind _asbp_player_state (Utilities|Casting|CastToBP_PlayerState (Variables|/Script/Engine.Controller|GetPlayerState _playercontroller)))
  (Default|CollectTaxes _asbp_player_state)
  (Default|ClientStartTurn _playercontroller))

(event Custom|BuildPhaseBegin
  ;[1 1 1] Build phase
  (bind _outactors (Actor|GetAllActorsOfClass "/Game/Blueprints/Player/BP_PlayerController.BP_PlayerController_C"))
  (for _array_element _outactors
    (Default|ClientBuildPhaseBegin _array_element)))

(event Custom|BuildPhaseEnd
  (bind _playercontroller (Utilities|PlayerinTurn))
  (bind _playercontroller_2 (Utilities|PlayerinTurn))
  (bind _playercontroller_3 (Utilities|PlayerNotinTurn))
  ;[1 1 1] Build phase
  (bind _output_get (Variables|Default|SetPlayersReady (+ 1 (Variables|Default|GetPlayersReady))))
  (if (== _output_get 2)
    (bind _returnvalue (Game|SpawnActorfromClass "/Game/Blueprints/Player/BP_Player.BP_Player_C" (Transformation|GetActorTransform (.Value (Utilities|Map|Find (Variables|Default|GetSpawnPoints) (Default|GetPlayerIndex _playercontroller)))) "AlwaysSpawn" _playercontroller 0))
    (Actor|DestroyActor (Pawn|GetControlledPawn _playercontroller_2))
    (Pawn|Possess _playercontroller_2 _returnvalue)
    (bind _returnvalue_2 (Game|SpawnActorfromClass "/Game/Blueprints/Player/BP_Player.BP_Player_C" (Transformation|GetActorTransform (.Value (Utilities|Map|Find (Variables|Default|GetSpawnPoints) (Default|GetPlayerIndex (Utilities|PlayerNotinTurn))))) "AlwaysSpawn" 0 0))
    (Actor|DestroyActor (Pawn|GetControlledPawn _playercontroller_3))
    (Pawn|Possess _playercontroller_3 _returnvalue_2)
    (CallFunction|StartGame)))

(event Custom|EndGame
  ;[1 1 1] End game
  (Utilities|FlowControl|Delay 5.0)
  (Game|OpenLevel(byName) "MainMenuLevel"))

(event Custom|UpdateWindStrength
  ;[1 1 1] Wind gameplay
  (bind _output_get (Variables|Default|SetNewRandomStrength (+ (CallFunction|GetWindStrength) (Math|Random|RandomFloatinRange -2e+01 2e+01))))
  (bind _newtrack_0 (Timeline|WindIncrease PlayFromStart)
    (:Update
      (Variables|Default|SetWindStrength (Math|Float|Lerp (CallFunction|GetWindStrength) _output_get _newtrack_0)))))

(event Custom|UpdateWindDirection
  (bind _returnvalue (Math|Random|RandomFloatinRange -1.0 1.0))
  (bind _winddirection (Variables|Default|GetWindDirection))
  ;[1 1 1] Wind gameplay
  (bind _output_get (Variables|Default|SetNewRandomWind (Math|Vector|MakeVector (+ _returnvalue (.x _winddirection)) (+ _returnvalue (.y _winddirection)) (.z _winddirection))))
  (bind _newtrack_0 (Timeline|Timeline_0 PlayFromStart)
    (:Update
      (Variables|Default|SetWindDirectionNormalized (Math|Vector|Normalize (Math|Vector|Lerp(Vector) (Variables|Default|GetWindDirection) _output_get _newtrack_0))))))

(event EventPostLogin
  (params (NewPlayer :type Player%20Controller%20Object%20Reference))
  ;[1 1 1] Game setup
  (bind _returnvalue (Class|GameModeBase|GetNumPlayers))
  (bind _asbp_player_controller (Utilities|Casting|CastToBP_PlayerController NewPlayer))
  (Default|SetPlayerIndex _asbp_player_controller (- _returnvalue 1))
  (bind _returnvalue_2 (Class|GameModeBase|GetNumPlayers))
  (if (== _returnvalue_2 2)
    (Utilities|FlowControl|Delay 1.0)
    (CallFunction|BuildPhaseBegin)
    (CallFunction|RandomizeWindDirection)
    (CallFunction|RandomizeWindStrength)))

(fn ConstructionScript)

(fn ChoosePlayerStart
  (params (Player :type Controller%20Object%20Reference))
  (CallFunction|InitializeSpawnPoints)
  (bind _returnvalue (Class|GameModeBase|GetNumPlayers))
  (return (.Value (Utilities|Map|Find (Variables|Default|GetSpawnPoints) _returnvalue))))

(fn InitializeSpawnPoints
  (if (== (Utilities|Map|Length (Variables|Default|GetSpawnPoints)) 0)
    (bind _outactors (Actor|GetAllActorsOfClass "/Game/Blueprints/Player/BP_PlayerStart.BP_PlayerStart_C"))
    (for _array_element _outactors
      (Utilities|Map|Add (Variables|Default|GetSpawnPoints) (Default|GetPlayerIndex _array_element) _array_element))))

(fn RandomizeWindDirection
  (bind _randomwinddirectionmin (LocalVariables|GetRandomWindDirectionMin))
  (bind _randomwinddirectionmax (LocalVariables|GetRandomWindDirectionMax))
  (bind _output_get (Variables|Default|SetWindDirection (Math|Vector|MakeVector (Math|Random|RandomFloatinRange (.x _randomwinddirectionmin) (.x _randomwinddirectionmax)) (Math|Random|RandomFloatinRange (.y _randomwinddirectionmin) (.y _randomwinddirectionmax)) (Math|Random|RandomFloatinRange (.z _randomwinddirectionmin) (.z _randomwinddirectionmax)))))
  (Variables|Default|SetWindDirectionNormalized (Math|Vector|Normalize (Math|Vector|MakeVector (.x _output_get) (.y _output_get) (.z _output_get)))))

(fn RandomizeWindStrength
  (Variables|Default|SetWindStrength (Math|Random|RandomFloatinRange (LocalVariables|GetRandomWindStrengthMin) (LocalVariables|GetRandomWindStrengthMax))))

(fn GetWindStrength
  (return (Variables|Default|GetWindStrength)))

(fn GetWindDirectionNormalized
  (return (Variables|Default|GetWindDirectionNormalized)))

(fn GetWindForce
  (return (* (Variables|Default|GetWindDirectionNormalized) (Variables|Default|GetWindStrength))))