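; Player character Blueprint that handles camera-relative movement and look, run/idle camera shakes, and a player index taken from its controller.
; Each tick, a camera line trace highlights the aimed-at handle or button on a BP_TrebuchetCurrent through custom depth.
; Up and Down keys use a sphere trace to raise or lower a nearby BP_TrebuchetOld's projectile mass and print the result.
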(event EventBeginPlay
  (bind _asbp_player_controller (Utilities|Casting|CastToBP_PlayerController (Pawn|GetController)))
  (CallFunction|SetPlayerIndex (Default|GetPlayerIndex _asbp_player_controller))
  (bind _outactors (Actor|GetAllActorsOfClass "/Game/Blueprints/BP_Screen.BP_Screen_C")))

(event EventTick
  (params (DeltaSeconds :type Float%20%28single-precision%29))
  (bind _playercamera (Variables|Default|GetPlayerCamera))
  (bind _returnvalue (Transformation|GetWorldLocation _playercamera))
  ;[1 1 1] Highlight Interraction points
  (bind (_outhit _returnvalue_2) (Collision|LineTraceByChannel _returnvalue (+ _returnvalue (* (Math|Vector|GetForwardVector (Transformation|GetWorldRotation _playercamera)) "500.000000,500.000000,500.000000")) "TraceTypeQuery1" false 0 "None" true "(R=1.000000,G=0.000000,B=0.000000,A=1.000000)" "(R=0.000000,G=1.000000,B=0.000000,A=1.000000)" 0.5))
  (if _returnvalue_2
    (if (Actor|ActorHasTag (.HitActor (Collision|BreakHitResult _outhit)) "Trebuchet")
      (bind _output_get (Variables|Default|SetTest (.HitActor (Collision|BreakHitResult _outhit))))
      (bind _asbp_trebuchet_current (Utilities|Casting|CastToBP_TrebuchetCurrent _output_get))
      (bind _array_element (Utilities|Array|ForEachLoopwithBreak (Utilities|Array|MakeArray (Variables|/Game/Blueprints/BP_TrebuchetCurrent.BP_TrebuchetCurrent_C|GetFireHandle _asbp_trebuchet_current) (Variables|/Game/Blueprints/BP_TrebuchetCurrent.BP_TrebuchetCurrent_C|GetReloadHandle _asbp_trebuchet_current) (Variables|/Game/Blueprints/BP_TrebuchetCurrent.BP_TrebuchetCurrent_C|GetSM_RotationHandle _asbp_trebuchet_current) (Variables|/Game/Blueprints/BP_TrebuchetCurrent.BP_TrebuchetCurrent_C|GetSM_WeightControll_IncreaseButton _asbp_trebuchet_current) (Variables|/Game/Blueprints/BP_TrebuchetCurrent.BP_TrebuchetCurrent_C|GetSM_WeightControll_DecreaseButton _asbp_trebuchet_current)) :!label _label)
        (:LoopBody
          (if (== _array_element (.HitComponent (Collision|BreakHitResult _outhit)))
            (Rendering|SetRenderCustomDepth _array_element true)
            (goto _label Break)
            (else
              (Rendering|SetRenderCustomDepth _array_element false)))))
      (else
        (bind _asbp_trebuchet_current_2 (Utilities|Casting|CastToBP_TrebuchetCurrent (Variables|Default|GetTest) :!label _label_2))
        (Rendering|SetRenderCustomDepth (Variables|/Game/Blueprints/BP_TrebuchetCurrent.BP_TrebuchetCurrent_C|GetFireHandle _asbp_trebuchet_current_2) false)))
    (else
      (goto _label_2))))

(event Input|AxisEvents|InputAxisLook
  (params (AxisValue :type Float%20%28single-precision%29))
  ;[1 1 1] Player Rotation
  (Pawn|Input|AddControllerPitchInput (Math|Float|Clamp(Float) AxisValue -2.0 2.0)))

(event Input|AxisEvents|InputAxisTurn
  (params (AxisValue :type Float%20%28single-precision%29))
  ;[1 1 1] Player Rotation
  (Pawn|Input|AddControllerYawInput (Math|Float|Clamp(Float) AxisValue -2.0 2.0)))

(event Input|AxisEvents|InputAxisMove
  (params (AxisValue :type Float%20%28single-precision%29))
  (bind _playerindex (Variables|Default|GetPlayerIndex))
  (bind _returnvalue (Game|GetPlayerCameraManager _playerindex))
  ;[1 1 1] Player Movement
  (Pawn|Input|AddMovementInput (Math|Vector|GetForwardVector (Math|Rotator|MakeRotator 0.0 0.0 (.Yaw (Math|Rotator|BreakRotator (Pawn|GetControlRotation :!class /Script/Engine.Pawn))))) AxisValue false)
  (if (> (Math|Vector|VectorLength (Transformation|GetVelocity)) 1e+02)
    (Class|MatineeCameraShake|StartMatineeCameraShake _returnvalue "/Game/Blueprints/Player/RunCameraShake.RunCameraShake_C" 1.0 "CameraLocal" "0, 0, 0")
    (elif (not (AI|Components|NavMovement|IsFalling (Variables|Character|GetCharacterMovement)))
      (Class|MatineeCameraShake|StartMatineeCameraShake _returnvalue "/Game/Blueprints/Player/IdleCameraShake.IdleCameraShake_C" 1.0 "CameraLocal" "0, 0, 0"))))

(event Input|AxisEvents|InputAxisStrafe
  (params (AxisValue :type Float%20%28single-precision%29))
  ;[1 1 1] Player Movement
  (Pawn|Input|AddMovementInput (Math|Vector|GetRightVector (Math|Rotator|MakeRotator 0.0 0.0 (.Yaw (Math|Rotator|BreakRotator (Pawn|GetControlRotation :!class /Script/Engine.Pawn))))) AxisValue false))

(event Input|KeyboardEvents|Up
  (params (Key :type Key%20Structure :default "None"))
  (bind _capsulecomponent (Variables|Collision|GetCapsuleComponent))
  (bind _massmodifier (Variables|Default|GetMassModifier))
  (bind _returnvalue (Transformation|GetWorldLocation _capsulecomponent))
  (:Pressed
    (Variables|Default|SetMoreMass true)
    (bind _outhits (Collision|MultiSphereTraceForObjects _returnvalue _returnvalue 5e+02 (Utilities|Array|MakeArray "ObjectTypeQuery2") false 0 "None"))
    (bind _array_element (Utilities|Array|ForEachLoopwithBreak _outhits :!label _label)
      (:LoopBody
        (bind _asbp_trebuchet_old (Utilities|Casting|CastToBP_TrebuchetOld (.HitActor (Collision|BreakHitResult _array_element))))
        (if (Variables|Default|GetMoreMass)
          (Class|PrimitiveComponent|SetMassOverrideinKg (Variables|/Game/Blueprints/BP_TrebuchetOld.BP_TrebuchetOld_C|GetSM_Projectile _asbp_trebuchet_old) "None" (+ (Physics|GetMass (Variables|/Game/Blueprints/BP_TrebuchetOld.BP_TrebuchetOld_C|GetSM_Projectile _asbp_trebuchet_old)) _massmodifier) true)
          (else
            (Class|PrimitiveComponent|SetMassOverrideinKg (Variables|/Game/Blueprints/BP_TrebuchetOld.BP_TrebuchetOld_C|GetSM_Projectile _asbp_trebuchet_old) "None" (- (Physics|GetMass (Variables|/Game/Blueprints/BP_TrebuchetOld.BP_TrebuchetOld_C|GetSM_Projectile _asbp_trebuchet_old)) _massmodifier) true)))
        (Development|PrintString (Utilities|String|ToString(Float) (Physics|GetMass (Variables|/Game/Blueprints/BP_TrebuchetOld.BP_TrebuchetOld_C|GetSM_Projectile _asbp_trebuchet_old))))
        (goto _label Break)))))

(event Input|KeyboardEvents|Down
  (params (Key :type Key%20Structure :default "None"))
  (bind _capsulecomponent (Variables|Collision|GetCapsuleComponent))
  (bind _massmodifier (Variables|Default|GetMassModifier))
  (bind _returnvalue (Transformation|GetWorldLocation _capsulecomponent))
  (:Pressed
    (Variables|Default|SetMoreMass false)
    (bind _outhits (Collision|MultiSphereTraceForObjects _returnvalue _returnvalue 5e+02 (Utilities|Array|MakeArray "ObjectTypeQuery2") false 0 "None"))
    (bind _array_element (Utilities|Array|ForEachLoopwithBreak _outhits :!label _label)
      (:LoopBody
        (bind _asbp_trebuchet_old (Utilities|Casting|CastToBP_TrebuchetOld (.HitActor (Collision|BreakHitResult _array_element))))
        (if (Variables|Default|GetMoreMass)
          (Class|PrimitiveComponent|SetMassOverrideinKg (Variables|/Game/Blueprints/BP_TrebuchetOld.BP_TrebuchetOld_C|GetSM_Projectile _asbp_trebuchet_old) "None" (+ (Physics|GetMass (Variables|/Game/Blueprints/BP_TrebuchetOld.BP_TrebuchetOld_C|GetSM_Projectile _asbp_trebuchet_old)) _massmodifier) true)
          (else
            (Class|PrimitiveComponent|SetMassOverrideinKg (Variables|/Game/Blueprints/BP_TrebuchetOld.BP_TrebuchetOld_C|GetSM_Projectile _asbp_trebuchet_old) "None" (- (Physics|GetMass (Variables|/Game/Blueprints/BP_TrebuchetOld.BP_TrebuchetOld_C|GetSM_Projectile _asbp_trebuchet_old)) _massmodifier) true)))
        (Development|PrintString (Utilities|String|ToString(Float) (Physics|GetMass (Variables|/Game/Blueprints/BP_TrebuchetOld.BP_TrebuchetOld_C|GetSM_Projectile _asbp_trebuchet_old))))
        (goto _label Break)))))

(fn ConstructionScript)

(fn GetPlayerIndex
  (return (Variables|Default|GetPlayerIndex)))

(fn SetPlayerIndex
  (params (NewParam :type Integer))
  (Variables|Default|SetPlayerIndex NewParam))