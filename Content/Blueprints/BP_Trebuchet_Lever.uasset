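; BP_Trebuchet_Lever is an interactable lever that fires or reloads the BP_TrebuchetOld it is attached to.
; TriggerInterraction casts the attach parent to the trebuchet, then calls CallFire or CallReload according to InterractionType and prints a debug message.
; Both actions play the AnimateLever timeline, which rolls the handle mesh through its pull.
; The construction script writes the Text variable to the lever's text label.
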(event EventTriggerInterraction
  (bind _asbp_trebuchet (Utilities|Casting|CastToBP_TrebuchetOld (Actor|GetAttachParentActor)))
  (switch Utilities|FlowControl|Switch|SwitchonE_LeverType (Variables|LeverSettings|GetInterraction%20Type)
    (:NewEnumerator0
      (Default|CallFire _asbp_trebuchet)
      (Development|PrintString "Launch Trebuchet" true true "(R=0.681645,G=1.000000,B=0.000000,A=1.000000)")
      (bind _pull_lever (Timeline|Animate%20Lever PlayFromStart)
        (:Update
          (Transformation|SetRelativeRotation (Variables|Default|GetSM_Lever_Handle) (Math|Rotator|MakeRotator (* _pull_lever 9e+01) 0.0 0.0) false false))))
    (:NewEnumerator1
      (Default|CallReload _asbp_trebuchet)
      (Development|PrintString "Reload Trebuchet" true true "(R=0.681644,G=1.000000,B=0.000000,A=1.000000)")
      (Timeline|Animate%20Lever PlayFromStart))))

(fn ConstructionScript
  (Rendering|Components|TextRender|SetText (Variables|Default|GetTextRender) (Variables|LeverSettings|GetText)))