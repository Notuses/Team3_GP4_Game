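; BP_TempProjectile is a projectile that deals area damage to buildings and sets off a destruction explosion on hit.
; Its Hit event sphere-traces around the impact, damages each BP_Building found, and enables physics on the Geometry Collection of those at zero health.
; It then spawns an FS_ExplodeField_Explosion field actor with the same radius and a strain magnitude, triggers it, and destroys itself.
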(event Collision|EventHit
  (params (MyComp :type Primitive%20Component%20Object%20Reference) (Other :type Actor%20Object%20Reference) (OtherComp :type Primitive%20Component%20Object%20Reference) (bSelfMoved :type Boolean) (HitLocation :type Vector :default "0, 0, 0") (HitNormal :type Vector :default "0, 0, 0") (NormalImpulse :type Vector :default "0, 0, 0") (Hit :type Hit%20Result%20Structure%20%28by%20ref%29))
  (bind _radius (Variables|Default|GetRadius))
  (bind _outhits (Collision|MultiSphereTraceForObjects HitLocation HitLocation _radius (Utilities|Array|MakeArray "ObjectTypeQuery7") false 0 (Variables|Default|GetDraw%20Debug%20Type) true "(R=1.000000,G=0.000000,B=0.000000,A=1.000000)" "(R=0.000000,G=1.000000,B=0.000000,A=1.000000)" (Variables|Default|GetDraw%20Time)))
  (for _array_element _outhits
    (if (Utilities|IsValid (.HitActor (Collision|BreakHitResult _array_element)))
      (bind _asbp_building (Utilities|Casting|CastToBP_Building (.HitActor (Collision|BreakHitResult _array_element))))
      (Default|TakeDamage _asbp_building (Variables|Default|GetDamage))
      (if (<= (Variables|/Game/Blueprints/Buildings/BP_Building.BP_Building_C|GetHealth _asbp_building) 0.0)
        (Default|DestroyCollisionBox _asbp_building)
        (Physics|SetSimulatePhysics (Variables|/Game/Blueprints/Buildings/BP_Building.BP_Building_C|GetGeoCollection _asbp_building) true))))
  (bind _returnvalue (Game|SpawnActorfromClass "/Game/GeometryCollections/FS_ExplodeField_Explosion.FS_ExplodeField_Explosion_C" (Math|Transform|MakeTransform HitLocation "0, 0, 0" "1.000000,1.000000,1.000000") "Undefined" 0 0))
  (Default|SetExplodeRadius _returnvalue _radius)
  (Default|SetExplosionStrainMagnitude _returnvalue (Variables|Default|GetStrainMagnitude))
  (Default|Explode _returnvalue)
  (Actor|DestroyActor))

(fn ConstructionScript)